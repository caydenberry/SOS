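; Acid bubble effect actor that plays a repeating bubble pop sound at its location.
; On BeginPlay it stays hidden for a configurable InitDelay, then shows itself and starts PlayFX.
; PlayFX loops endlessly through delay nodes, firing the sound cue at the root component's position every few seconds.
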(event `playFX`
  ;[1 1 1] Makes bubble sound go pop
  (`KismetSystemLibrary.Delay` 3.0 :!label _label)
  (`KismetSystemLibrary.Delay` 1.0)
  (`GameplayStatics.PlaySoundAtLocation` "/Game/assets/sounds/acid/bubble_soundcue.bubble_soundcue" (`SceneComponent.K2_GetComponentLocation` (`self.DefaultSceneRoot`)))
  (goto _label))

(event `self.ReceiveBeginPlay`
  ;[1 1 1] Makes bubble sound go pop
  (`self.SetActorHiddenInGame` true)
  (`KismetSystemLibrary.Delay` (`self.initDelay`))
  (`self.SetActorHiddenInGame` false)
  (`self.playFX`))

(fn `UserConstructionScript`)