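; Large ceiling floodlight Blueprint whose lit state follows a referenced power switch.
; Every tick it casts the switch reference to PowerSwitch, reads its Power flag and calls TurnOn or TurnOff.
; Those events swap the floodlight mesh's second material slot between lit and off materials and show or hide the point light.
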(event `Turn On`
  ;[1 1 1] Turn On
  (`PrimitiveComponent.SetMaterial` (`self.floodlight_ceiling`) 1 "/Game/assets/materials/light_white.light_white")
  (`SceneComponent.SetVisibility` (`self.PointLight`) true false))

(event `Turn Off`
  ;[1 1 1] Turn Off
  (`PrimitiveComponent.SetMaterial` (`self.floodlight_ceiling`) 1 "/Game/assets/materials/light_off.light_off")
  (`SceneComponent.SetVisibility` (`self.PointLight`) false false))

(event `self.ReceiveTick`
  (params (DeltaSeconds :type "Float (single-precision)"))
  ;[1 1 1] Lights
  (bind _aspower_switch (cast `/Game/assets/blueprints/Interactables/PowerSwitch` (`self.PowerSwitch`)))
  (set `self.Power` (`/Game/assets/blueprints/Interactables/PowerSwitch.Power` _aspower_switch))
  (if (`self.Power`)
    (`self.Turn On`)
    (else
      (`self.Turn Off`))))

(fn `UserConstructionScript`)