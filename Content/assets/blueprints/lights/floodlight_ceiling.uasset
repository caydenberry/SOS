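; Ceiling floodlight actor for the medbay that lights up or goes dark depending on a linked power switch.
; Every tick it casts its PowerSwitch reference and reads that switch's Power flag to call TurnOn or TurnOff.
; Those events swap the bulb material on the fixture mesh between lit and unlit versions and toggle the point light's visibility.
; The state is polled and reapplied each frame rather than driven by change events.
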(event `Turn On`
  ;[1 1 1] Turn On
  (`PrimitiveComponent.SetMaterial` (`self.floodlight_ceiling`) 1 "/Game/assets/materials/medbay_floodlight_ceiling_bulb.medbay_floodlight_ceiling_bulb")
  (`SceneComponent.SetVisibility` (`self.PointLight`) true false))

(event `Turn Off`
  ;[1 1 1] Turn Off
  (`PrimitiveComponent.SetMaterial` (`self.floodlight_ceiling`) 1 "/Game/assets/materials/medbay_floodlight_ceiling_bulb_off.medbay_floodlight_ceiling_bulb_off")
  (`SceneComponent.SetVisibility` (`self.PointLight`) false false))

(event `self.ReceiveTick`
  (params (DeltaSeconds :type "Float (single-precision)"))
  ;[1 1 1] Lights
  (bind _aspower_switch (cast `/Game/assets/blueprints/Interactables/PowerSwitch` (`self.PowerSwitch`)))
  (set `self.Power` (`/Game/assets/blueprints/Interactables/PowerSwitch.Power` _aspower_switch))
  (if (`self.Power`)
    (`self.Turn On`)
    (else
      (`self.Turn Off`))))

(fn `UserConstructionScript`)