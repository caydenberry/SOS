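; Medbay button door that the first-person player opens and closes by interacting while overlapping it, if power is on and, when locked, the backpack holds the required key.
; Tick reads power from a PowerSwitch and sets lights and panel materials for unpowered, locked or unlocked states.
; ShiftDoor polls for interaction through a Delay loop, slides the door with MoveComponentTo and switches the lights between green (closed) and yellow (open).
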(event `CloseDoor`
  ;[1 1 1] Door Is Opened Or Closed
  (`KismetSystemLibrary.MoveComponentTo` (`self.medbay_door`) (`SceneComponent.RelativeLocation` (`self.DoorClosed`))))

(event `OpenDoor`
  ;[1 1 1] Door Is Opened Or Closed
  (`KismetSystemLibrary.MoveComponentTo` (`self.medbay_door`) (`SceneComponent.RelativeLocation` (`self.DoorOpen`))))

(event `PowerOff`
  ;[1 1 1] Power Off Setup
  (`SceneComponent.SetVisibility` (`self.PointLight`) false false)
  (`SceneComponent.SetVisibility` (`self.PointLight1`) false false)
  (`PrimitiveComponent.SetMaterial` (`self.medbay_door_frame`) 1 "/Game/assets/materials/light_off.light_off")
  (`PrimitiveComponent.SetMaterial` (`self.door_panel`) 2 "/Game/assets/materials/light_off.light_off")
  (`PrimitiveComponent.SetMaterial` (`self.door_panel2`) 2 "/Game/assets/materials/alpha_grate.alpha_grate")
  (`PrimitiveComponent.SetMaterial` (`self.door_panel`) 1 "/Game/assets/materials/light_off.light_off")
  (`PrimitiveComponent.SetMaterial` (`self.door_panel2`) 1 "/Game/assets/materials/alpha_grate.alpha_grate")
  (set `self.init` true)
  (set `self.firstUnlocked` true))

(event `self.ReceiveBeginPlay`
  ;[1 1 1] Open or Closed Initially
  (if (`self.Open`)
    (`self.OpenDoor`)
    (else
      (`self.CloseDoor`)))
  (bind _aspower_switch (cast `/Game/assets/blueprints/Interactables/PowerSwitch` (`self.powerSwitchClass`))
    (:`then`
      (bind _outactors (`GameplayStatics.GetAllActorsWithTag` (`self.doorname`))))
    (:`CastFailed`
      (`KismetSystemLibrary.PrintString` "fail"))))

(event `LockedDoor`
  ;[1 1 1] Locked Door Setup
  (`LightComponent.SetLightColor` (`self.PointLight`) (struct :`R` 0.390625 :`B` 0.001963 :`A` 1.0) true)
  (`LightComponent.SetLightColor` (`self.PointLight1`) (struct :`R` 0.390625 :`B` 0.001963 :`A` 1.0) true)
  (`PrimitiveComponent.SetMaterial` (`self.medbay_door_frame`) 1 "/Game/assets/materials/light_red.light_red")
  (`PrimitiveComponent.SetMaterial` (`self.door_panel`) 2 "/Game/assets/materials/light_red.light_red")
  (`PrimitiveComponent.SetMaterial` (`self.door_panel2`) 2 "/Game/assets/materials/light_red.light_red")
  (set `self.firstLocked` false)
  (set `self.firstUnlocked` true))

(event `self.ReceiveActorBeginOverlap`
  (params (OtherActor :type "Actor Object Reference"))
  ;[1 1 1] Prompt and Trigger
  (`KismetSystemLibrary.PrintString` "\"Press E to Open Door\"")
  (`self.ShiftDoor`)
  (set `self.isOverlapping` true))

(event `self.ReceiveTick`
  (params (DeltaSeconds :type "Float (single-precision)"))
  ;[1 1 1] Locked Door Functionality
  (`/Engine/EditorBlueprintResources/StandardMacros.IsValid` (`|GetArrayItem` (stale `self.ReceiveBeginPlay` _outactors))
    (:`Is Valid`
      (set `self.Power` (`/Game/assets/blueprints/Interactables/PowerSwitch.Power` (stale `self.ReceiveBeginPlay` _aspower_switch)))
      (if (`self.Power`)
        (`SceneComponent.SetVisibility` (`self.PointLight`) true false)
        (`SceneComponent.SetVisibility` (`self.PointLight1`) true false)
        (if (`self.isLocked`)
          (if (`self.firstLocked`)
            (`self.LockedDoor`)
            (set `self.init` false))
          (elif (`self.firstUnlocked`)
            (`self.Unlocked Door`)
            (set `self.init` false)
            (elif (`self.init`)
              (`PrimitiveComponent.SetMaterial` (`self.medbay_door_frame`) 1 "/Game/assets/materials/light_green.light_green")
              (set `self.init` false))))
        (else
          (`self.PowerOff`))))
    (:`Is Not Valid`
      (`KismetSystemLibrary.PrintString` "meddoorfail"))))

(event `Unlocked Door`
  ;[1 1 1] Unlocked Door Setup
  (`LightComponent.SetLightColor` (`self.PointLight`) (struct :`R` 0.003922 :`G` 0.211765 :`A` 1.0) true)
  (`LightComponent.SetLightColor` (`self.PointLight1`) (struct :`R` 0.003922 :`G` 0.211765 :`A` 1.0) true)
  (`PrimitiveComponent.SetMaterial` (`self.medbay_door_frame`) 1 "/Game/assets/materials/light_green.light_green")
  (`PrimitiveComponent.SetMaterial` (`self.door_panel`) 2 "/Game/assets/materials/light_green.light_green")
  (`PrimitiveComponent.SetMaterial` (`self.door_panel2`) 2 "/Game/assets/materials/light_green.light_green")
  (set `self.firstLocked` true)
  (set `self.firstUnlocked` false))

(event `self.ReceiveActorEndOverlap`
  (params (OtherActor :type "Actor Object Reference"))
  ;[1 1 1] Prompt and Trigger
  (set `self.isOverlapping` false))

(event `ShiftDoor`
  (bind _door_panel2 (`self.door_panel2`))
  (bind _door_panel (`self.door_panel`))
  (bind _pointlight (`self.PointLight`))
  (bind _pointlight1 (`self.PointLight1`))
  (bind _medbay_door_frame (`self.medbay_door_frame`))
  ;[1 1 1] Door Open and Close
  (bind _asfirst_person_character (cast `/Game/FirstPersonBP/Blueprints/FirstPersonCharacter` (stale `self.ReceiveActorBeginOverlap` OtherActor))
    (:`then`
      _)
    (:`CastFailed`
      (`KismetSystemLibrary.PrintString` "cast failed")))
  (if (`/Game/FirstPersonBP/Blueprints/FirstPersonCharacter.isInteracting` _asfirst_person_character) :!label _label
    (if (`self.Power`)
      (if (`self.isLocked`)
        (if (`KismetArrayLibrary.Array_Contains` (`/Game/assets/blueprints/BaseInventory.NameList` (`|GetArrayItem` (`/Game/FirstPersonBP/Blueprints/FirstPersonCharacter.Backpack` _asfirst_person_character) (`self.slot`))) (`self.KeyRequired`))
          (if (`self.Open`) :!label _label_2
            (`self.CloseDoor`)
            (set `self.Open` false)
            ;;[1 1 1] Changes Light Color
            (`LightComponent.SetLightColor` _pointlight (struct :`R` 0.003922 :`G` 0.211765 :`A` 1.0) true)
            (`LightComponent.SetLightColor` _pointlight1 (struct :`R` 0.003922 :`G` 0.211765 :`A` 1.0) true)
            (`PrimitiveComponent.SetMaterial` _medbay_door_frame 1 "/Game/assets/materials/light_green.light_green")
            (`PrimitiveComponent.SetMaterial` _door_panel 2 "/Game/assets/materials/light_green.light_green")
            (`PrimitiveComponent.SetMaterial` _door_panel2 2 "/Game/assets/materials/light_green.light_green")
            (else
              (`self.OpenDoor`)
              (set `self.Open` true)
              (`LightComponent.SetLightColor` _pointlight (struct :`R` 0.395833 :`G` 0.388174 :`B` 0.12922 :`A` 1.0) true)
              (`LightComponent.SetLightColor` _pointlight1 (struct :`R` 0.395833 :`G` 0.388174 :`B` 0.12922 :`A` 1.0) true)
              (`PrimitiveComponent.SetMaterial` _medbay_door_frame 1 "/Game/assets/materials/light_yellow.light_yellow")
              (`PrimitiveComponent.SetMaterial` _door_panel 2 "/Game/assets/materials/light_yellow.light_yellow")
              (`PrimitiveComponent.SetMaterial` _door_panel2 2 "/Game/assets/materials/light_yellow.light_yellow")))
          (if (`self.isOverlapping`)
            (`KismetSystemLibrary.Delay` 0.1 :!label _label_3)
            (if (`/Game/FirstPersonBP/Blueprints/FirstPersonCharacter.overlapPlayer` _asfirst_person_character)
              (if (`/Game/FirstPersonBP/Blueprints/FirstPersonCharacter.alreadyOverlapped` _asfirst_person_character) :!label _label_4
                (`KismetSystemLibrary.Delay` 0.1)
                (goto _label_4)
                (elif (`self.isOverlapping`)
                  (goto _label)))))
          (else
            (set `self.slot` 0)
            (`KismetSystemLibrary.PrintString` "Door Is Locked")
            (goto _label_3)))
        (else
          (goto _label_2)))
      (else
        (goto _label_3)))
    (else
      (goto _label_3))))

(fn `UserConstructionScript`)