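; Obstacle shooter that repeatedly fires projectiles while its linked PowerSwitch is on.
; Tick copies the switch's power state, and a looping BeginPlay chain polls it, applying a one-time startup delay before firing at a set interval.
; Each shot spawns the projectile at ProjectileSpawn, sets its Direction opposite the actor's forward vector, plays a fire sound and animates the Shaft out and back.
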(event `self.ReceiveBeginPlay`
  ;[1 1 1] Overall Loop
  (if (`self.Power`) :!label _label
    (if (`self.Init`)
      (`KismetSystemLibrary.Delay` (`self.SecondsUntilStartup`))
      (set `self.Init` false))
    (`self.Shoot`)
    (`KismetSystemLibrary.Delay` (`self.SecondsPerShot`))
    (goto _label)
    (else
      (`KismetSystemLibrary.Delay` 0.1)
      (goto _label))))

(event `Shoot`
  (bind _shaft (`self.Shaft`))
  ;[1 1 1] ShootLoop
  (bind _asprojectile (castclass `/Game/assets/blueprints/Obstacles/Projectile` "/Game/assets/blueprints/Obstacles/Projectile.Projectile_C")
    (:`then`
      (bind _returnvalue (`|SpawnActorFromClass` _asprojectile (`SceneComponent.K2_GetComponentToWorld` (`self.ProjectileSpawn`)) "AlwaysSpawn" "OverrideRootScale" null null))
      (set `/Game/assets/blueprints/Obstacles/Projectile.direction` (* (`self.GetActorForwardVector` self) (-10000.0 -10000.0 -10000.0)) _returnvalue)
      (`GameplayStatics.PlaySoundAtLocation` "/Game/FirstPerson/Audio/FirstPersonTemplateWeaponFire02_Cue.FirstPersonTemplateWeaponFire02_Cue" (`SceneComponent.K2_GetComponentLocation` (`self.Body`)) (struct) 0.25)
      (`KismetSystemLibrary.MoveComponentTo` _shaft (45.0 0.0 0.0) (struct) false false 0.1)
      (`KismetSystemLibrary.MoveComponentTo` _shaft (-45.0 0.0 0.0) (struct) false false 0.5))
    (:`CastFailed`
      (`KismetSystemLibrary.PrintString` "Fail"))))

(event `self.ReceiveTick`
  (params (DeltaSeconds :type "Float (single-precision)"))
  ;[1 1 1] Checking Tick
  (set `self.Power` (`/Game/assets/blueprints/Interactables/PowerSwitch.Power` (`self.PowerSwitch`))))

(fn `UserConstructionScript`)