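; Stomper obstacle that repeatedly rises and slams down, killing the first-person player caught beneath it.
; After an initial configurable delay, BeginPlay runs an endless latent loop that slowly lifts the static mesh, dips it slightly as a tell, then drops it quickly to its relative origin.
; The Activated flag is set only during the drop, and KillTrig overlaps beginning in that window set PlayerHealth to zero.
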(event `self.ReceiveBeginPlay`
  (bind _staticmesh (`self.StaticMesh`))
  (`KismetSystemLibrary.Delay` (`self.delay`))
  (`KismetSystemLibrary.MoveComponentTo` _staticmesh (0.0 0.0 1000.0) (struct) false false 3.5 :!label _label)
  (`KismetSystemLibrary.Delay` 2.0)
  (`KismetSystemLibrary.MoveComponentTo` _staticmesh (0.0 0.0 980.0))
  (`KismetSystemLibrary.Delay` 1.25)
  (set `self.Activated` true)
  (`KismetSystemLibrary.MoveComponentTo` _staticmesh (0.0 0.0 0.0) (struct) false false 0.65)
  (set `self.Activated` false)
  (`KismetSystemLibrary.Delay` 3.0)
  (goto _label))

(event `self.KillTrig.OnComponentBeginOverlap`
  (params (OverlappedComponent :type "PrimitiveComponent Object Reference") (OtherActor :type "Actor Object Reference") (OtherComp :type "PrimitiveComponent Object Reference") (OtherBodyIndex :type Integer) (bFromSweep :type Boolean) (SweepResult :type "HitResult Structure (by ref)"))
  (bind _asfirst_person_character (cast `/Game/FirstPersonBP/Blueprints/FirstPersonCharacter` OtherActor)
    (:`then`
      (if (`self.Activated`)
        (set `/Game/FirstPersonBP/Blueprints/FirstPersonCharacter.player_health` 0 _asfirst_person_character)))
    (:`CastFailed`
      (`KismetSystemLibrary.PrintString` "Stomper Fail"))))

(fn `UserConstructionScript`)