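; Obstacle projectile actor that damages and launches the first-person player on overlap.
; Shortly after spawning, its sphere gets a velocity-change impulse built from direction, multiplier and an added vector.
; Player hits reduce health, set a launch force from sphere forward and direction, then destroy the projectile.
; Other overlaps print a failure and route into the same delayed self-destruct that limits its lifetime.
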(event `self.ReceiveBeginPlay`
  (bind _multiplier (`self.multiplier`))
  (bind _returnvalue (+ (* (`self.direction`) _multiplier) (`self.vectorAdd`)))
  ;[1 1 1] Killing off all copies
  (`KismetSystemLibrary.Delay` 0.01)
  (`PrimitiveComponent.AddImpulse` (`self.Sphere`) _returnvalue "None" true)
  (`KismetSystemLibrary.PrintString` (`KismetStringLibrary.Conv_VectorToString` _returnvalue))
  (`KismetSystemLibrary.PrintString` (`KismetStringLibrary.Conv_DoubleToString` _multiplier))
  (`KismetSystemLibrary.Delay` 10.0 :!label _label)
  (`self.K2_DestroyActor`))

(event `self.ReceiveActorBeginOverlap`
  (params (OtherActor :type "Actor Object Reference"))
  ;[1 1 1] Projectile
  (bind _asfirst_person_character (cast `/Game/FirstPersonBP/Blueprints/FirstPersonCharacter` OtherActor)
    (:`then`
      (set `/Game/FirstPersonBP/Blueprints/FirstPersonCharacter.player_health` (- (`/Game/FirstPersonBP/Blueprints/FirstPersonCharacter.player_health` _asfirst_person_character) (`self.damage`)) _asfirst_person_character)
      (set `/Game/FirstPersonBP/Blueprints/FirstPersonCharacter.LaunchForce` (/ (* (`KismetMathLibrary.GetForwardVector` (`SceneComponent.K2_GetComponentRotation` (`self.Sphere`))) (`self.direction`)) (10.0 10.0 10.0)) _asfirst_person_character)
      (set `/Game/FirstPersonBP/Blueprints/FirstPersonCharacter.IsLaunched` true _asfirst_person_character)
      (`self.K2_DestroyActor`))
    (:`CastFailed`
      (`KismetSystemLibrary.PrintString` "fail")
      (goto _label))))

(fn `UserConstructionScript`)