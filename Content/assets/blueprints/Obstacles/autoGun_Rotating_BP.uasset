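; Rotating auto-gun obstacle that fires endless bursts of projectiles from its SpawnPoint.
; BeginPlay loops on Delays, spawning BurstSize shots at a pace set by FireRatePerSecond, pausing between bursts and toggling IsShooting on the gun's anim Blueprint.
; Each projectile's Direction is the scaled, negated actor forward vector; a random-rotation spread branch is left disconnected.
; Tick turns Center by a fixed step per frame, so rotation speed depends on frame rate.
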(event `self.ReceiveBeginPlay`
  ;[1 1 1] AutoGun
  (bind _asprojectile (castclass `/Game/assets/blueprints/Obstacles/Projectile` "/Game/assets/blueprints/Obstacles/Projectile.Projectile_C"))
  (bind _asauto_gun_anim_bp (cast `/Game/assets/models/animated/autoGun/autoGun_animBP` (`SkeletalMeshComponent.GetAnimInstance` (`self.autoMesh`)))
    (:`then`
      (set `/Game/assets/models/animated/autoGun/autoGun_animBP.location` (`SceneComponent.K2_GetComponentLocation` (`self.SpawnPoint`)) _asauto_gun_anim_bp)
      (if (< (`self.i`) (`self.burstSize`)) :!label _label
        (`KismetSystemLibrary.PrintString` (`KismetStringLibrary.Conv_IntToString` (`self.i`)))
        (set `/Game/assets/models/animated/autoGun/autoGun_animBP.isShooting` true _asauto_gun_anim_bp)
        (set `self.i` (+ (`self.i`) 1))
        (bind _returnvalue (`|SpawnActorFromClass` _asprojectile (`SceneComponent.K2_GetComponentToWorld` (`self.SpawnPoint`)) "Undefined" "OverrideRootScale" null null))
        (set `/Game/assets/blueprints/Obstacles/Projectile.direction` (* (`self.GetActorForwardVector` self) (-10000.0 -10000.0 -10000.0)) _returnvalue)
        (`KismetSystemLibrary.Delay` 0.083)
        (set `/Game/assets/models/animated/autoGun/autoGun_animBP.isShooting` false _asauto_gun_anim_bp)
        (`KismetSystemLibrary.Delay` (/ (/ 1.0 (`self.FireRatePerSecond`)) 2.0))
        (goto _label)
        (else
          (`KismetSystemLibrary.Delay` (`self.SecondsBetweenBursts`))
          (set `self.i` 0)
          (goto _label))))
    (:`CastFailed`
      (`KismetSystemLibrary.PrintString` "autoGunFail"))))

(event `self.ReceiveTick`
  (params (DeltaSeconds :type "Float (single-precision)"))
  ;[1 1 1] Rotation
  (`SceneComponent.K2_AddRelativeRotation` (`self.Center`) (struct :`Pitch` 0.2) false false))

(fn `UserConstructionScript`)