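; Base item actor that the first-person character can pick up, prompted on screen as a keycard.
; Construction script sets its mesh from a MeshChoice-indexed lookup.
; On overlap, Delay loops poll the character's overlap and interact flags, then add the item to its Backpack and mark it picked up.
; End overlap clears IsOverlapping, which gates the pickup.
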(event `self.ReceiveActorBeginOverlap`
  (params (OtherActor :type "Actor Object Reference"))
  ;[1 1 1] Pick Up Keycard
  (set `self.isOverlapping` true)
  (bind _asfirst_person_character (cast `/Game/FirstPersonBP/Blueprints/FirstPersonCharacter` OtherActor))
  (`KismetSystemLibrary.PrintString` "\"Press E to pick up Keycard\"")
  (if (`/Game/FirstPersonBP/Blueprints/FirstPersonCharacter.overlapPlayer` _asfirst_person_character) :!label _label
    (if (`/Game/FirstPersonBP/Blueprints/FirstPersonCharacter.alreadyOverlapped` _asfirst_person_character) :!label _label_2
      (`KismetSystemLibrary.Delay` 0.1)
      (goto _label_2)
      (elif (`self.isOverlapping`)
        (if (`/Game/FirstPersonBP/Blueprints/FirstPersonCharacter.isInteracting` _asfirst_person_character)
          (`/Game/assets/blueprints/BaseInventory.AddItemToInventory` (`/Game/FirstPersonBP/Blueprints/FirstPersonCharacter.Backpack` _asfirst_person_character) self)
          (set `self.isPickedUp` true)
          (else
            (`KismetSystemLibrary.Delay` 0.1)
            (goto _label)))))))

(event `self.ReceiveActorEndOverlap`
  (params (OtherActor :type "Actor Object Reference"))
  ;[1 1 1] Leave Area
  (set `self.isOverlapping` false))

(fn `UserConstructionScript`
  (locals (NewLocalVar_0 :type "Array of StaticMesh Object Reference"))
  (`StaticMeshComponent.SetStaticMesh` (`self.ItemMesh`) (`|GetArrayItem` (`local.NewLocalVar_0`) (`KismetMathLibrary.Conv_ByteToInt` (`self.MeshChoice`)))))