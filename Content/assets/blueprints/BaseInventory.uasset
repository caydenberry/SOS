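; BaseInventory is an actor Blueprint that stores picked actors in an inventory list.
; AddItemToInventory wraps the incoming actor in an InventorySlot struct with the slot count and name list, then appends it to ItemList.
; It records the actor's name in a parallel NameList, destroys the actor despite the slot referencing it, and returns the new index.
; Debug prints show the name, first list entry and index.
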(fn `AddItemToInventory`
  (params (`In Actor` :type "/Game/assets/blueprints/BaseItem Object Reference"))
  (returns (Slot :type Integer))
  (bind _name (`/Game/assets/blueprints/BaseItem.Name` `In Actor`))
  (bind _namelist (`self.NameList`))
  (bind _returnvalue (`KismetArrayLibrary.Array_Add` (`self.ItemList`) (make `/Game/assets/blueprints/InventorySlot` (`|MakeArray` `In Actor`) (`self.SlotCount`) (`self.NameList`))))
  (`KismetSystemLibrary.PrintString` (`KismetStringLibrary.BuildString_Name` "" "" _name))
  (`KismetArrayLibrary.Array_Add` _namelist _name)
  (bind _output_get (set `self.IndexAdded` _returnvalue))
  (`KismetSystemLibrary.PrintString` (`KismetStringLibrary.Conv_NameToString` (`|GetArrayItem` _namelist)))
  (`self.K2_DestroyActor` `In Actor`)
  (`KismetSystemLibrary.PrintString` (`KismetStringLibrary.BuildString_Int` "" "" _output_get))
  (return _output_get))

(fn `UserConstructionScript`)