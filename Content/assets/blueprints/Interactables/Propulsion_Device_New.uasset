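; Interactable propulsion device that launches the first-person character when they interact while overlapping it.
; BeginPlay pitches an arrow to the configured Angle and finds the character; Tick polls the overlap and interaction flags to fire Propulsion.
; Propulsion derives a vector from the arrow's forward direction and the Base-to-Shoot offset, scales it by Power, then writes the character's LaunchForce and IsLaunched, leaving the launch to that character.
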(event `self.ReceiveBeginPlay`
  ;[1 1 1] Initial Lights Settings
  (`KismetSystemLibrary.MoveComponentTo` (`self.Arrow`) (0.0 0.0 0.0) (`KismetMathLibrary.MakeRotator` 0.0 (`self.angle`)))
  (bind _outactors (`GameplayStatics.GetAllActorsOfClass` "/Game/FirstPersonBP/Blueprints/FirstPersonCharacter.FirstPersonCharacter_C")))

(event `self.ReceiveActorBeginOverlap`
  (params (OtherActor :type "Actor Object Reference"))
  ;[1 1 1] Trigger
  (cast `/Game/FirstPersonBP/Blueprints/FirstPersonCharacter` OtherActor)
  (set `self.IsOverlapped` true))

(event `Propulsion`
  (bind _returnvalue (- (`SceneComponent.K2_GetComponentLocation` (`self.shoot`)) (`SceneComponent.K2_GetComponentLocation` (`self.base`))))
  (bind _returnvalue_2 (* (* (`KismetMathLibrary.GetForwardVector` (`SceneComponent.K2_GetComponentRotation` (`self.Arrow`))) _returnvalue) _returnvalue))
  ;[1 1 1] Propulsion
  (`/Engine/EditorBlueprintResources/StandardMacros.CompareFloat` (`self.power`)
    (:`>`
      (`KismetSystemLibrary.PrintString` (`KismetStringLibrary.Conv_VectorToString` _returnvalue_2)))
    (:`==`
      (set `self.power` 0.0 :!label _label))
    (:`<`
      (goto _label)))
  (bind _output (`|GetArrayItem` (stale `self.ReceiveBeginPlay` _outactors)))
  (set `/Game/FirstPersonBP/Blueprints/FirstPersonCharacter.LaunchForce` (* (/ (* _returnvalue_2 (-5.0 -5.0 1.0)) (20.0 20.0 20.0)) (`self.power`)) _output)
  (set `/Game/FirstPersonBP/Blueprints/FirstPersonCharacter.IsLaunched` true _output)
  (`KismetSystemLibrary.Delay` 2.0))

(event `self.ReceiveActorEndOverlap`
  (params (OtherActor :type "Actor Object Reference"))
  ;[1 1 1] Trigger
  (set `self.IsOverlapped` false))

(event `self.ReceiveTick`
  (params (DeltaSeconds :type "Float (single-precision)"))
  ;[1 1 1] Setup
  (bind _output (`|GetArrayItem` (stale `self.ReceiveBeginPlay` _outactors)))
  (`/Engine/EditorBlueprintResources/StandardMacros.IsValid` _output
    (:`Is Valid`
      (if (`/Game/FirstPersonBP/Blueprints/FirstPersonCharacter.PlayerBodyOverlap` _output)
        (if (`/Game/FirstPersonBP/Blueprints/FirstPersonCharacter.alreadyOverlapped` _output)
          _
          (elif (`self.IsOverlapped`)
            (if (`/Game/FirstPersonBP/Blueprints/FirstPersonCharacter.isInteracting` _output)
              (`self.Propulsion`))))))))

(fn `UserConstructionScript`)