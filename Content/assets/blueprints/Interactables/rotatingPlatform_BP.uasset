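; Rotating platform interactable that passes four rotation requests to its animation blueprint.
; On BeginPlay it caches the RotatingPlatform_AnimBP from the Platform mesh's anim instance.
; Tick polls Rotate1 to Rotate4 in priority order, sets the matching AnimBP flag and clears its own.
; The AnimBP flag is cleared within the same tick, except Rotate3, which stays true.
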(event `self.ReceiveBeginPlay`
  ;[1 1 1] Casts to animbp
  (bind _asrotating_platform_anim_bp (cast `/Game/assets/models/animated/RotatePlatform/RotatingPlatform_AnimBP` (`SkeletalMeshComponent.GetAnimInstance` (`self.Platform`)))))

(event `self.ReceiveTick`
  (params (DeltaSeconds :type "Float (single-precision)"))
  ;[1 1 1] Rotation
  (if (`self.rotate1`)
    (set `/Game/assets/models/animated/RotatePlatform/RotatingPlatform_AnimBP.rotate1` true (stale `self.ReceiveBeginPlay` _asrotating_platform_anim_bp))
    (set `self.rotate1` false)
    (set `/Game/assets/models/animated/RotatePlatform/RotatingPlatform_AnimBP.rotate1` false (stale `self.ReceiveBeginPlay` _asrotating_platform_anim_bp))
    (elif (`self.rotate2`)
      (set `/Game/assets/models/animated/RotatePlatform/RotatingPlatform_AnimBP.rotate2` true (stale `self.ReceiveBeginPlay` _asrotating_platform_anim_bp))
      (set `self.rotate2` false)
      (set `/Game/assets/models/animated/RotatePlatform/RotatingPlatform_AnimBP.rotate2` false (stale `self.ReceiveBeginPlay` _asrotating_platform_anim_bp))
      (elif (`self.rotate3`)
        (set `/Game/assets/models/animated/RotatePlatform/RotatingPlatform_AnimBP.rotate3` true (stale `self.ReceiveBeginPlay` _asrotating_platform_anim_bp))
        (set `self.rotate3` false)
        (set `/Game/assets/models/animated/RotatePlatform/RotatingPlatform_AnimBP.rotate3` true (stale `self.ReceiveBeginPlay` _asrotating_platform_anim_bp))
        (elif (`self.rotate4`)
          (set `/Game/assets/models/animated/RotatePlatform/RotatingPlatform_AnimBP.rotate4` true (stale `self.ReceiveBeginPlay` _asrotating_platform_anim_bp))
          (set `self.rotate4` false)
          (set `/Game/assets/models/animated/RotatePlatform/RotatingPlatform_AnimBP.rotate4` false (stale `self.ReceiveBeginPlay` _asrotating_platform_anim_bp)))))))

(fn `UserConstructionScript`)