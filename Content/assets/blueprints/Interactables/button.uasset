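; Floor-style button actor that unlocks a linked medbay door when the first-person character overlaps it.
; BeginPlay casts the Door reference to the medbay button door, with a debug print shared by both failed casts.
; Overlap sets IsPressed, turns the button green and moves it down.
; Tick writes the door's locked state from IsPressed every frame; nothing here resets the press.
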(event `self.ReceiveBeginPlay`
  ;[1 1 1] Casting to the Door
  (bind _asmedbay_button_door (cast `/Game/assets/blueprints/doors/medbay_button_door` (`self.Door`))
    (:`CastFailed`
      ;[1 1 1] Pree Button
      (`KismetSystemLibrary.PrintString` "FAIL BITCH" :!label _label))))

(event `self.ReceiveActorBeginOverlap`
  (params (OtherActor :type "Actor Object Reference"))
  (bind _button (`self.button`))
  ;[1 1 1] Pree Button
  (cast `/Game/FirstPersonBP/Blueprints/FirstPersonCharacter` OtherActor
    (:`then`
      (set `self.isPressed` true)
      (`PrimitiveComponent.SetMaterial` _button 1 "/Game/assets/materials/light_green.light_green")
      (`KismetSystemLibrary.MoveComponentTo` _button (0.0 0.0 -20.0)))
    (:`CastFailed`
      (goto _label))))

(event `self.ReceiveTick`
  (params (DeltaSeconds :type "Float (single-precision)"))
  ;[1 1 1] Changing the door's states.
  (if (`self.isPressed`)
    (set `/Game/assets/blueprints/doors/medbay_button_door.isLocked` false (stale `self.ReceiveBeginPlay` _asmedbay_button_door))
    (else
      (set `/Game/assets/blueprints/doors/medbay_button_door.isLocked` true (stale `self.ReceiveBeginPlay` _asmedbay_button_door)))))

(fn `UserConstructionScript`)