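; Interactable vent piece, named as a dead end, that the FirstPersonCharacter can pick up, carry, drop and throw.
; Overlap starts a Delay-based polling loop that checks the character's overlap flags and toggles holding and mesh physics on interact.
; While held, Tick snaps the mesh to the character's PickUp component, and firing launches it with a camera-forward impulse.
; Ending overlap releases it and enables physics.
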(event `self.ReceiveBeginPlay`
  ;[1 1 1] SONOVABITCH
  (`PrimitiveComponent.SetSimulatePhysics` (`self.StaticMesh`) false))

(event `self.ReceiveActorBeginOverlap`
  (params (OtherActor :type "Actor Object Reference"))
  (bind _staticmesh (`self.StaticMesh`))
  ;[1 1 1] SONOVABITCH
  (bind _asfirst_person_character (cast `/Game/FirstPersonBP/Blueprints/FirstPersonCharacter` OtherActor)
    (:`then`
      (set `self.isOverlapping` true)
      (if (`/Game/FirstPersonBP/Blueprints/FirstPersonCharacter.overlapPlayer` _asfirst_person_character) :!label _label
        (if (`/Game/FirstPersonBP/Blueprints/FirstPersonCharacter.alreadyOverlapped` _asfirst_person_character) :!label _label_2
          (`KismetSystemLibrary.Delay` 0.1)
          (goto _label_2)
          (elif (`self.isOverlapping`)
            (if (`/Game/FirstPersonBP/Blueprints/FirstPersonCharacter.isInteracting` _asfirst_person_character)
              (if (`/Game/FirstPersonBP/Blueprints/FirstPersonCharacter.isHoldingItem` _asfirst_person_character)
                (if (`self.isPickedUp`)
                  (set `self.isPickedUp` false)
                  (`PrimitiveComponent.SetSimulatePhysics` _staticmesh true)
                  (set `/Game/FirstPersonBP/Blueprints/FirstPersonCharacter.isHoldingItem` false _asfirst_person_character)
                  (`KismetSystemLibrary.Delay` 0.1 :!label _label_3)
                  (goto _label)
                  (else
                    (`KismetSystemLibrary.PrintString` "error")))
                (else
                  (set `self.isPickedUp` true)
                  (`PrimitiveComponent.SetSimulatePhysics` _staticmesh false)
                  (set `/Game/FirstPersonBP/Blueprints/FirstPersonCharacter.isHoldingItem` true _asfirst_person_character)
                  (goto _label_3)))
              (else
                (goto _label_3)))
            (else
              (set `self.isOverlapping` false :!label _label_4)
              (set `/Game/FirstPersonBP/Blueprints/FirstPersonCharacter.isHoldingItem` false _asfirst_person_character)
              (set `self.isPickedUp` false)
              (`PrimitiveComponent.SetSimulatePhysics` _staticmesh true))))
        (else
          (goto _label_4))))
    (:`CastFailed`
      (`KismetSystemLibrary.PrintString` "Cast Failed")
      (goto _label_4))))

(event `self.ReceiveActorEndOverlap`
  (params (OtherActor :type "Actor Object Reference"))
  ;[1 1 1] SONOVABITCH
  (goto _label_4))

(event `self.ReceiveTick`
  (params (DeltaSeconds :type "Float (single-precision)"))
  (bind _staticmesh (`self.StaticMesh`))
  ;[1 1 1] SONOVABITCH
  (if (`self.isPickedUp`)
    (if (`/Game/FirstPersonBP/Blueprints/FirstPersonCharacter.isFiring` (stale `self.ReceiveActorBeginOverlap` _asfirst_person_character))
      (set `self.isPickedUp` false)
      (set `/Game/FirstPersonBP/Blueprints/FirstPersonCharacter.isHoldingItem` false (stale `self.ReceiveActorBeginOverlap` _asfirst_person_character))
      (`PrimitiveComponent.SetSimulatePhysics` _staticmesh true)
      (bind _returnvalue (`KismetMathLibrary.GetForwardVector` (`SceneComponent.K2_GetComponentRotation` (`/Game/FirstPersonBP/Blueprints/FirstPersonCharacter.FirstPersonCamera` (stale `self.ReceiveActorBeginOverlap` _asfirst_person_character)))))
      (`PrimitiveComponent.AddImpulse` (`self.StaticMesh`) (* (+ (+ (0.0 0.0 0.0) _returnvalue) _returnvalue) (10000.0 10000.0 10000.0)) "None" false)
      (else
        (`SceneComponent.K2_SetWorldLocation` _staticmesh (`SceneComponent.K2_GetComponentLocation` (`/Game/FirstPersonBP/Blueprints/FirstPersonCharacter.PickUp` (stale `self.ReceiveActorBeginOverlap` _asfirst_person_character))) false false)))))

(fn `UserConstructionScript`)