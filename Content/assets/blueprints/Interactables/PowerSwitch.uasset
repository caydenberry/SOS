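; PowerSwitch is an interactable switch actor that the first-person character toggles between powered and unpowered.
; Overlap events track the player's presence, while Tick polls the character's interaction and overlap flags to flip Power.
; Each flip updates the PowerSwitch_animbp animation Blueprint, and AnimTransition with a Delay blocks retriggering during the transition.
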(event `self.ReceiveBeginPlay`
  ;[1 1 1] Casting to the AnimBP
  (bind _aspower_switch_animbp (cast `/Game/assets/models/animated/powerswitch/PowerSwitch_animbp` (`SkeletalMeshComponent.GetAnimInstance` (`self.PowerSwitch`))))
  (set `/Game/assets/models/animated/powerswitch/PowerSwitch_animbp.Power` (`self.Power`) _aspower_switch_animbp)
  (bind _outactors (`GameplayStatics.GetAllActorsOfClass` "/Game/FirstPersonBP/Blueprints/FirstPersonCharacter.FirstPersonCharacter_C" :!label _label)))

(event `self.ReceiveActorBeginOverlap`
  (params (OtherActor :type "Actor Object Reference"))
  ;[1 1 1] Setup
  (cast `/Game/FirstPersonBP/Blueprints/FirstPersonCharacter` OtherActor)
  (set `self.isOverlapped` true)
  (goto _label))

(event `self.ReceiveActorEndOverlap`
  (params (OtherActor :type "Actor Object Reference"))
  ;[1 1 1] Setup
  (set `self.isOverlapped` false))

(event `self.ReceiveTick`
  (params (DeltaSeconds :type "Float (single-precision)"))
  ;[1 1 1] Interaction
  (bind _output (`|GetArrayItem` (stale `self.ReceiveBeginPlay` _outactors)))
  (`/Engine/EditorBlueprintResources/StandardMacros.IsValid` _output
    (:`Is Valid`
      (if (`self.AnimTransition`)
        _
        (elif (`/Game/FirstPersonBP/Blueprints/FirstPersonCharacter.overlapPlayer` _output)
          (if (`/Game/FirstPersonBP/Blueprints/FirstPersonCharacter.alreadyOverlapped` _output)
            _
            (elif (`self.IsOverlapped`)
              (if (`/Game/FirstPersonBP/Blueprints/FirstPersonCharacter.isInteracting` _output)
                (if (`self.Power`)
                  (set `self.Power` false)
                  (else
                    (set `self.Power` true)))
                (set `/Game/assets/models/animated/powerswitch/PowerSwitch_animbp.Power` (`self.Power`) (stale `self.ReceiveBeginPlay` _aspower_switch_animbp))
                (set `self.AnimTransition` true)
                (`KismetSystemLibrary.Delay` 1.0)
                (set `self.AnimTransition` false)))))))))

(fn `UserConstructionScript`)