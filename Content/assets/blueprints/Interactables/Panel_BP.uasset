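; Interactable panel that lets the first-person player step a linked ChildRotator through four rotation states.
; On overlap, it re-checks the character's OverlapPlayer and IsInteracting flags in a Delay loop, advancing one state on each poll while interaction is active.
; The state cycles through the Rotate1 to Rotate4 booleans, starting at Rotate1 when none is set.
; The loop ends with a debug print once OverlapPlayer is false.
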(event `self.ReceiveBeginPlay`)

(event `self.ReceiveActorBeginOverlap`
  (params (OtherActor :type "Actor Object Reference"))
  (bind _childrotator (`self.childRotator`))
  (bind _asfirst_person_character (cast `/Game/FirstPersonBP/Blueprints/FirstPersonCharacter` OtherActor))
  (if (`/Game/FirstPersonBP/Blueprints/FirstPersonCharacter.overlapPlayer` _asfirst_person_character) :!label _label
    (if (`/Game/FirstPersonBP/Blueprints/FirstPersonCharacter.isInteracting` _asfirst_person_character)
      (if (`/Game/assets/blueprints/Interactables/rotatingPlatform_BP.rotate4` _childrotator)
        (set `/Game/assets/blueprints/Interactables/rotatingPlatform_BP.rotate1` true _childrotator)
        (set `/Game/assets/blueprints/Interactables/rotatingPlatform_BP.rotate4` false _childrotator)
        (elif (`/Game/assets/blueprints/Interactables/rotatingPlatform_BP.rotate1` _childrotator)
          (set `/Game/assets/blueprints/Interactables/rotatingPlatform_BP.rotate2` true _childrotator)
          (set `/Game/assets/blueprints/Interactables/rotatingPlatform_BP.rotate1` false _childrotator)
          (elif (`/Game/assets/blueprints/Interactables/rotatingPlatform_BP.rotate2` _childrotator)
            (set `/Game/assets/blueprints/Interactables/rotatingPlatform_BP.rotate3` true _childrotator)
            (set `/Game/assets/blueprints/Interactables/rotatingPlatform_BP.rotate2` false _childrotator)
            (elif (`/Game/assets/blueprints/Interactables/rotatingPlatform_BP.rotate3` _childrotator)
              (set `/Game/assets/blueprints/Interactables/rotatingPlatform_BP.rotate4` true _childrotator)
              (set `/Game/assets/blueprints/Interactables/rotatingPlatform_BP.rotate3` false _childrotator)
              (else
                (set `/Game/assets/blueprints/Interactables/rotatingPlatform_BP.rotate1` true _childrotator)))))))
    (`KismetSystemLibrary.Delay` 0.1)
    (goto _label)
    (else
      (`KismetSystemLibrary.PrintString` "Ah Fuck"))))

(fn `UserConstructionScript`)