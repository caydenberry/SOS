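; Interactable propulsion device that launches the first-person character when they interact inside its trigger.
; BeginPlay tilts the body to Angle and caches the character; Tick polls overlap and interaction flags to fire Propulsion.
; Propulsion writes a Power-scaled LaunchForce, derived from Base-to-Shoot offset and unit facing, and IsLaunched onto the character.
; The unit snaps to Shoot, then slowly retracts, with lights switching red, yellow and green by phase.
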(event `self.ReceiveBeginPlay`
  (bind _propulsion_lights (`self.Propulsion_Lights`))
  ;[1 1 1] Initial Lights Settings
  (`PrimitiveComponent.SetMaterial` _propulsion_lights 1 "/Game/assets/materials/light_green.light_green")
  (`PrimitiveComponent.SetMaterial` _propulsion_lights 2 "/Game/assets/materials/light_green.light_green")
  (`PrimitiveComponent.SetMaterial` _propulsion_lights 3 "/Game/assets/materials/light_green.light_green")
  (`KismetSystemLibrary.MoveComponentTo` (`self.Propulsion_Body`) (0.0 0.0 0.0) (`KismetMathLibrary.MakeRotator` 0.0 (`self.angle`)) false false 0.1)
  (bind _outactors (`GameplayStatics.GetAllActorsOfClass` "/Game/FirstPersonBP/Blueprints/FirstPersonCharacter.FirstPersonCharacter_C")))

(event `self.Trigger.OnComponentBeginOverlap`
  (params (OverlappedComponent :type "PrimitiveComponent Object Reference") (OtherActor :type "Actor Object Reference") (OtherComp :type "PrimitiveComponent Object Reference") (OtherBodyIndex :type Integer) (bFromSweep :type Boolean) (SweepResult :type "HitResult Structure (by ref)"))
  ;[1 1 1] Trigger
  (cast `/Game/FirstPersonBP/Blueprints/FirstPersonCharacter` OtherActor)
  (set `self.IsOverlapped` true))

(event `Propulsion`
  (bind _propulsion_lights (`self.Propulsion_Lights`))
  (bind _propulsion_lights_2 (`self.Propulsion_Lights`))
  (bind _propulsion_lights_3 (`self.Propulsion_Lights`))
  (bind _returnvalue (- (`SceneComponent.K2_GetComponentLocation` (`self.Shoot`)) (`SceneComponent.K2_GetComponentLocation` (`self.Base`))))
  ;[1 1 1] Propulsion
  (`PrimitiveComponent.SetMaterial` _propulsion_lights 1 "/Game/assets/materials/light_red.light_red")
  (`PrimitiveComponent.SetMaterial` _propulsion_lights 2 "/Game/assets/materials/light_red.light_red")
  (`PrimitiveComponent.SetMaterial` _propulsion_lights 3 "/Game/assets/materials/light_red.light_red")
  (`/Engine/EditorBlueprintResources/StandardMacros.CompareFloat` (`self.power`)
    (:`>`
      _)
    (:`==`
      (set `self.power` 0.0 :!label _label))
    (:`<`
      (goto _label)))
  (bind _output (`|GetArrayItem` (stale `self.ReceiveBeginPlay` _outactors)))
  (set `/Game/FirstPersonBP/Blueprints/FirstPersonCharacter.LaunchForce` (* (/ (* (* _returnvalue (* (`KismetMathLibrary.GetForwardVector` (`SceneComponent.K2_GetComponentRotation` (`self.Propulsion_Unit`))) _returnvalue)) (-5.0 -5.0 -1.0)) (20.0 20.0 20.0)) (`self.power`)) _output)
  (`KismetSystemLibrary.PrintString` (`KismetStringLibrary.Conv_VectorToString` _returnvalue))
  (set `/Game/FirstPersonBP/Blueprints/FirstPersonCharacter.IsLaunched` true _output)
  (`KismetSystemLibrary.MoveComponentTo` (`self.Propulsion_Unit`) (`SceneComponent.RelativeLocation` (`self.Shoot`)) (struct) false false 0.05)
  (`KismetSystemLibrary.Delay` 2.0)
  (`PrimitiveComponent.SetMaterial` _propulsion_lights_3 1 "/Game/assets/materials/light_yellow.light_yellow")
  (`PrimitiveComponent.SetMaterial` _propulsion_lights_3 2 "/Game/assets/materials/light_yellow.light_yellow")
  (`PrimitiveComponent.SetMaterial` _propulsion_lights_3 3 "/Game/assets/materials/light_yellow.light_yellow")
  (`KismetSystemLibrary.MoveComponentTo` (`self.Propulsion_Unit`) (`SceneComponent.RelativeLocation` (`self.Base`)) (struct) false false 3.0)
  (`PrimitiveComponent.SetMaterial` _propulsion_lights_2 1 "/Game/assets/materials/light_green.light_green")
  (`PrimitiveComponent.SetMaterial` _propulsion_lights_2 2 "/Game/assets/materials/light_green.light_green")
  (`PrimitiveComponent.SetMaterial` _propulsion_lights_2 3 "/Game/assets/materials/light_green.light_green"))

(event `self.Trigger.OnComponentEndOverlap`
  (params (OverlappedComponent :type "PrimitiveComponent Object Reference") (OtherActor :type "Actor Object Reference") (OtherComp :type "PrimitiveComponent Object Reference") (OtherBodyIndex :type Integer))
  ;[1 1 1] Trigger
  (set `self.IsOverlapped` false))

(event `self.ReceiveTick`
  (params (DeltaSeconds :type "Float (single-precision)"))
  ;[1 1 1] Setup
  (bind _output (`|GetArrayItem` (stale `self.ReceiveBeginPlay` _outactors)))
  (`/Engine/EditorBlueprintResources/StandardMacros.IsValid` _output
    (:`Is Valid`
      (if (`/Game/FirstPersonBP/Blueprints/FirstPersonCharacter.overlapPlayer` _output)
        (if (`/Game/FirstPersonBP/Blueprints/FirstPersonCharacter.alreadyOverlapped` _output)
          _
          (elif (`self.IsOverlapped`)
            (if (`/Game/FirstPersonBP/Blueprints/FirstPersonCharacter.isInteracting` _output)
              (`self.Propulsion`))))))
    (:`Is Not Valid`
      (`KismetSystemLibrary.PrintString` "Failure"))))

(fn `UserConstructionScript`)