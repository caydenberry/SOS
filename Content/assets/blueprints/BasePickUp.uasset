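; Base pickup actor that lets the FirstPersonCharacter grab, carry, drop and throw a physics mesh.
; Box overlap starts a 0.1-second Delay loop polling the character's interact flag to toggle holding and physics simulation.
; While held, Tick snaps the mesh to the character's PickUp component, or launches it along camera forward when firing.
; End overlap or a failed cast clears the held state without re-enabling physics.
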(event `self.Box.OnComponentBeginOverlap`
  (params (OverlappedComponent :type "PrimitiveComponent Object Reference") (OtherActor :type "Actor Object Reference") (OtherComp :type "PrimitiveComponent Object Reference") (OtherBodyIndex :type Integer) (bFromSweep :type Boolean) (SweepResult :type "HitResult Structure (by ref)"))
  (bind _staticmesh (`self.StaticMesh`))
  ;[1 1 1] SONOVABITCH
  (bind _asfirst_person_character (cast `/Game/FirstPersonBP/Blueprints/FirstPersonCharacter` OtherActor)
    (:`then`
      (set `self.isOverlapping` true)
      (if (`self.isOverlapping`) :!label _label
        (if (`/Game/FirstPersonBP/Blueprints/FirstPersonCharacter.isInteracting` _asfirst_person_character)
          (if (`/Game/FirstPersonBP/Blueprints/FirstPersonCharacter.isHoldingItem` _asfirst_person_character)
            (if (`self.isPickedUp`)
              (set `self.isPickedUp` false)
              (`PrimitiveComponent.SetSimulatePhysics` _staticmesh true)
              (set `/Game/FirstPersonBP/Blueprints/FirstPersonCharacter.isHoldingItem` false _asfirst_person_character)
              (`KismetSystemLibrary.Delay` 0.1 :!label _label_2)
              (goto _label)
              (else
                (`KismetSystemLibrary.PrintString` "error")))
            (else
              (set `self.isPickedUp` true)
              (`PrimitiveComponent.SetSimulatePhysics` _staticmesh false)
              (set `/Game/FirstPersonBP/Blueprints/FirstPersonCharacter.isHoldingItem` true _asfirst_person_character)
              (goto _label_2)))
          (else
            (goto _label_2)))
        (else
          (set `self.isOverlapping` false :!label _label_3)
          (set `/Game/FirstPersonBP/Blueprints/FirstPersonCharacter.isHoldingItem` false _asfirst_person_character)
          (set `self.isPickedUp` false))))
    (:`CastFailed`
      (`KismetSystemLibrary.PrintString` "Cast Failed")
      (goto _label_3))))

(event `self.Box.OnComponentEndOverlap`
  (params (OverlappedComponent :type "PrimitiveComponent Object Reference") (OtherActor :type "Actor Object Reference") (OtherComp :type "PrimitiveComponent Object Reference") (OtherBodyIndex :type Integer))
  ;[1 1 1] SONOVABITCH
  (goto _label_3))

(event `self.ReceiveTick`
  (params (DeltaSeconds :type "Float (single-precision)"))
  (bind _staticmesh (`self.StaticMesh`))
  ;[1 1 1] SONOVABITCH
  (if (`self.isPickedUp`)
    (if (`/Game/FirstPersonBP/Blueprints/FirstPersonCharacter.isFiring` (stale `self.Box.OnComponentBeginOverlap` _asfirst_person_character))
      (set `self.isPickedUp` false)
      (set `/Game/FirstPersonBP/Blueprints/FirstPersonCharacter.isHoldingItem` false (stale `self.Box.OnComponentBeginOverlap` _asfirst_person_character))
      (`PrimitiveComponent.SetSimulatePhysics` _staticmesh true)
      (bind _returnvalue (`KismetMathLibrary.GetForwardVector` (`SceneComponent.K2_GetComponentRotation` (`/Game/FirstPersonBP/Blueprints/FirstPersonCharacter.FirstPersonCamera` (stale `self.Box.OnComponentBeginOverlap` _asfirst_person_character)))))
      (`PrimitiveComponent.AddImpulse` (`self.StaticMesh`) (* (+ (+ (0.0 0.0 0.0) _returnvalue) _returnvalue) (70000.0 70000.0 70000.0)) "None" false)
      (else
        (`SceneComponent.K2_SetWorldLocation` _staticmesh (`SceneComponent.K2_GetComponentLocation` (`/Game/FirstPersonBP/Blueprints/FirstPersonCharacter.PickUp` (stale `self.Box.OnComponentBeginOverlap` _asfirst_person_character))) false false)))))

(fn `UserConstructionScript`)