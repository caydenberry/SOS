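; Climbable ladder actor that lets an overlapping FirstPersonCharacter grab on, climb, drop or jump off.
; Overlap polls with Delay loops for interact input, then disables character movement and places LadderPosition at the player's height, clamped between TOP and BOTTOM.
; Tick pins the player to that component and reads character input flags to step it up or down.
; Reaching either end snaps and restores walking, while jumping hands a launch force to the character.
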(event `self.ReceiveBeginPlay`
  ;[1 1 1] Setup
  (set `self.TopFloat` (.z (`SceneComponent.K2_GetComponentLocation` (`self.TOP`))))
  (set `self.BottomFloat` (.z (`SceneComponent.K2_GetComponentLocation` (`self.BOTTOM`)))))

(event `self.ReceiveTick`
  (params (DeltaSeconds :type "Float (single-precision)"))
  ;[1 1 1] Tick
  (set `self.LadderPosZ` (.z (`SceneComponent.K2_GetComponentLocation` (`self.Ladder_Position`))))
  (if (`self.Init`)
    _
    (elif (`self.IsOnLadder`)
      (bind _rootcomponent (`Actor.RootComponent` (stale `self.ReceiveActorBeginOverlap` _asfirst_person_character)))
      (`SceneComponent.K2_SetWorldLocationAndRotation` _rootcomponent (`SceneComponent.K2_GetComponentLocation` (`self.Ladder_Position`)) (`SceneComponent.RelativeRotation` _rootcomponent) false false)
      (if (`/Game/FirstPersonBP/Blueprints/FirstPersonCharacter.isInteracting` (stale `self.ReceiveActorBeginOverlap` _asfirst_person_character))
        (`self.Drop`)
        (elif (`/Game/FirstPersonBP/Blueprints/FirstPersonCharacter.isJumping` (stale `self.ReceiveActorBeginOverlap` _asfirst_person_character))
          (`self.Launch`)
          (elif (`/Game/FirstPersonBP/Blueprints/FirstPersonCharacter.Wpressed` (stale `self.ReceiveActorBeginOverlap` _asfirst_person_character))
            (bind _spressed (`/Game/FirstPersonBP/Blueprints/FirstPersonCharacter.Spressed` (stale `self.ReceiveActorBeginOverlap` _asfirst_person_character)))
            (if (not _spressed)
              (`self.MoveUp`))
            (elif _spressed
              (`self.MoveDown`))))))))

(event `self.ReceiveActorBeginOverlap`
  (params (OtherActor :type "Actor Object Reference"))
  (bind _ladder_position (`self.Ladder_Position`))
  (bind _bottomfloat (`self.BottomFloat`))
  (bind _x (.x (`SceneComponent.K2_GetComponentLocation` (`self.BOTTOM`))))
  (bind _y (.y (`SceneComponent.K2_GetComponentLocation` (`self.BOTTOM`))))
  ;[1 1 1] Player Overlap Setup
  (bind _asfirst_person_character (cast `/Game/FirstPersonBP/Blueprints/FirstPersonCharacter` OtherActor))
  (set `self.isoverlapped` true)
  (if (`/Game/FirstPersonBP/Blueprints/FirstPersonCharacter.overlapPlayer` _asfirst_person_character) :!label _label
    (if (`/Game/FirstPersonBP/Blueprints/FirstPersonCharacter.alreadyOverlapped` _asfirst_person_character) :!label _label_2
      (`KismetSystemLibrary.Delay` 0.1)
      (goto _label_2)
      (elif (`/Game/FirstPersonBP/Blueprints/FirstPersonCharacter.isInteracting` _asfirst_person_character)
        (set `self.IsOnLadder` true)
        (bind _z (.z (`SceneComponent.K2_GetComponentLocation` (`Actor.RootComponent` _asfirst_person_character))))
        (`/Engine/EditorBlueprintResources/StandardMacros.CompareFloat` _z (`self.TopFloat`)
          (:`>`
            (bind _output_get (set `self.LadderPosZ` (`self.TopFloat`) :!label _label_3))
            (`SceneComponent.K2_SetWorldLocation` _ladder_position (`KismetMathLibrary.MakeVector` _x _y _output_get) false false))
          (:`==`
            (goto _label_3))
          (:`<`
            (`/Engine/EditorBlueprintResources/StandardMacros.CompareFloat` _z _bottomfloat
              (:`>`
                (bind _output_get_2 (set `self.LadderPosZ` _z))
                (`SceneComponent.K2_SetWorldLocation` _ladder_position (`KismetMathLibrary.MakeVector` _x _y _output_get_2) false false))
              (:`==`
                (bind _output_get_3 (set `self.LadderPosZ` _bottomfloat :!label _label_4))
                (`SceneComponent.K2_SetWorldLocation` _ladder_position (`KismetMathLibrary.MakeVector` _x _y _output_get_3) false false))
              (:`<`
                (goto _label_4)))))
        (`self.LadderBasics`)
        (`KismetSystemLibrary.Delay` 0.1)
        (set `self.Init` false)
        (else
          (`KismetSystemLibrary.Delay` 0.1)
          (goto _label))))))

(event `self.ReceiveActorEndOverlap`
  (params (OtherActor :type "Actor Object Reference"))
  ;[1 1 1] Player Overlap Setup
  (if (`self.IsOnLadder`) :!label _label_5
    (`KismetSystemLibrary.Delay` 0.1)
    (goto _label_5)
    (else
      (`self.Reset`))))

(event `Launch`
  ;[1 1 1] launch
  (`self.Reset`)
  (`self.LadderBasics`)
  (set `/Game/FirstPersonBP/Blueprints/FirstPersonCharacter.LaunchForce` (* (* (`KismetMathLibrary.GetForwardVector` (`SceneComponent.K2_GetComponentRotation` (`self.DefaultSceneRoot`))) (- (`SceneComponent.K2_GetComponentLocation` (`self.launchpos`)) (`SceneComponent.K2_GetComponentLocation` (`self.Ladder_Position`)))) (1000000.0 1000000.0 1000000.0)) (stale `self.ReceiveActorBeginOverlap` _asfirst_person_character))
  (set `/Game/FirstPersonBP/Blueprints/FirstPersonCharacter.IsLaunched` true (stale `self.ReceiveActorBeginOverlap` _asfirst_person_character)))

(event `MoveUp`
  (bind _ladder_position (`self.Ladder_Position`))
  ;[1 1 1] PlayerMoving
  (`/Engine/EditorBlueprintResources/StandardMacros.CompareFloat` (`self.LadderPosZ`) (`self.TopFloat`)
    (:`>`
      (set `self.isTop` true :!label _label_6)
      (`self.Snap`))
    (:`==`
      (goto _label_6))
    (:`<`
      (`KismetSystemLibrary.MoveComponentTo` _ladder_position (+ (`SceneComponent.RelativeLocation` _ladder_position) (0.0 0.0 5.0)) (struct) false false 0.05))))

(event `LadderBasics`
  ;[1 1 1] Ladder Basics
  (if (`self.IsOnLadder`)
    (bind _charactermovement (`Character.CharacterMovement` (stale `self.ReceiveActorBeginOverlap` _asfirst_person_character)))
    (`CharacterMovementComponent.SetMovementMode` _charactermovement "MOVE_None" 0)
    (else
      (`CharacterMovementComponent.SetMovementMode` _charactermovement "MOVE_Walking" 0))))

(event `Reset`
  ;[1 1 1] Reset
  (set `self.isoverlapped` false)
  (set `self.IsOnLadder` false)
  (set `self.Init` true)
  (set `self.isTop` false))

(event `MoveDown`
  (bind _ladder_position (`self.Ladder_Position`))
  ;[1 1 1] PlayerMoving
  (`/Engine/EditorBlueprintResources/StandardMacros.CompareFloat` (`self.LadderPosZ`) (`self.BottomFloat`)
    (:`>`
      (`KismetSystemLibrary.MoveComponentTo` _ladder_position (- (`SceneComponent.RelativeLocation` _ladder_position) (0.0 0.0 5.0)) (struct) false false 0.05))
    (:`==`
      (set `self.isTop` false :!label _label_7)
      (`self.Snap`))
    (:`<`
      (goto _label_7))))

(event `Drop`
  ;[1 1 1] Drop
  (set `self.IsOnLadder` false)
  (`self.Reset`)
  (`self.LadderBasics`))

(event `Snap`
  (bind _ladder_position (`self.Ladder_Position`))
  ;[1 1 1] Getting on and off of the ladder
  (if (`self.isTop`)
    (`KismetSystemLibrary.MoveComponentTo` _ladder_position (`SceneComponent.RelativeLocation` (`self.TopSnap`)))
    (else
      (`KismetSystemLibrary.MoveComponentTo` _ladder_position (`SceneComponent.RelativeLocation` (`self.BottomSnap`)))))
  (`self.Reset`)
  (`self.LadderBasics`))

(fn `UserConstructionScript`)