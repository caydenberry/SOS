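; Breakable floor actor that shatters when the FirstPersonCharacter overlaps it.
; The overlap event sets a Break flag, which Tick polls, using a Ticked flag so the break runs only once.
; The break destroys the intact floor mesh, reveals the hidden broken floor and pre-placed pieces, and enables physics simulation on the pieces.
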(event `self.ReceiveActorBeginOverlap`
  (params (OtherActor :type "Actor Object Reference"))
  ;[1 1 1] Allowing the place to break
  (bind _asfirst_person_character (cast `/Game/FirstPersonBP/Blueprints/FirstPersonCharacter` OtherActor)
    (:`then`
      (`/Engine/EditorBlueprintResources/StandardMacros.IsValid` _asfirst_person_character
        (:`Is Valid`
          (set `self.break` true))
        (:`Is Not Valid`
          (`KismetSystemLibrary.PrintString` "Is Invalid"))))
    (:`CastFailed`
      (`KismetSystemLibrary.PrintString` "Cast Failed"))))

(event `self.ReceiveTick`
  (params (DeltaSeconds :type "Float (single-precision)"))
  (bind _pieces06 (`self.pieces06`))
  (bind _pieces02 (`self.pieces02`))
  (bind _pieces03 (`self.pieces03`))
  (bind _pieces04 (`self.pieces04`))
  (bind _pieces05 (`self.pieces05`))
  (bind _pieces01 (`self.pieces01`))
  (bind _pieces07 (`self.pieces07`))
  (bind _pieces08 (`self.pieces08`))
  (bind _pieces09 (`self.pieces09`))
  (bind _pieces10 (`self.pieces10`))
  (bind _pieces11 (`self.pieces11`))
  ;[1 1 1] Break; make pieces spawn
  (if (`self.ticked`)
    _
    (elif (`self.break`)
      (`ActorComponent.K2_DestroyComponent` (`self.floor_regular`))
      (`SceneComponent.SetHiddenInGame` (`self.floor_broken`) false false)
      (`SceneComponent.SetHiddenInGame` _pieces01 false false)
      (`SceneComponent.SetHiddenInGame` _pieces02 false false)
      (`SceneComponent.SetHiddenInGame` _pieces03 false false)
      (`SceneComponent.SetHiddenInGame` _pieces04 false false)
      (`SceneComponent.SetHiddenInGame` _pieces05 false false)
      (`SceneComponent.SetHiddenInGame` _pieces06 false false)
      (`SceneComponent.SetHiddenInGame` _pieces07 false false)
      (`SceneComponent.SetHiddenInGame` _pieces08 false false)
      (`SceneComponent.SetHiddenInGame` _pieces09 false false)
      (`SceneComponent.SetHiddenInGame` _pieces10 false false)
      (`SceneComponent.SetHiddenInGame` _pieces11 false false)
      (`PrimitiveComponent.SetSimulatePhysics` _pieces01 true)
      (`PrimitiveComponent.SetSimulatePhysics` _pieces02 true)
      (`PrimitiveComponent.SetSimulatePhysics` _pieces03 true)
      (`PrimitiveComponent.SetSimulatePhysics` _pieces04 true)
      (`PrimitiveComponent.SetSimulatePhysics` _pieces05 true)
      (`PrimitiveComponent.SetSimulatePhysics` _pieces06 true)
      (`PrimitiveComponent.SetSimulatePhysics` _pieces07 true)
      (`PrimitiveComponent.SetSimulatePhysics` _pieces08 true)
      (`PrimitiveComponent.SetSimulatePhysics` _pieces09 true)
      (`PrimitiveComponent.SetSimulatePhysics` _pieces10 true)
      (`PrimitiveComponent.SetSimulatePhysics` _pieces11 true)
      (set `self.ticked` true))))

(fn `UserConstructionScript`)