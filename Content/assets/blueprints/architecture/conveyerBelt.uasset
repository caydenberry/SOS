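; Conveyor belt actor that pushes an overlapping FirstPersonCharacter along the forward vector of its BeltPlaceholder component.
; Begin and end overlap switch a force multiplier on and off, set the character's IsOnConveyerBelt flag and call its ConveyerBeltStatus.
; Tick applies the force to the CharacterMovement of the character from begin overlap every frame, without delta-time scaling or a validity check.
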(event `self.ReceiveActorBeginOverlap`
  (params (OtherActor :type "Actor Object Reference"))
  (bind _asfirst_person_character (cast `/Game/FirstPersonBP/Blueprints/FirstPersonCharacter` OtherActor))
  (set `self.forceMultiplier` 1000000)
  (set `/Game/FirstPersonBP/Blueprints/FirstPersonCharacter.isOnConveyerBelt` true _asfirst_person_character)
  (`/Game/FirstPersonBP/Blueprints/FirstPersonCharacter.conveyerBeltStatus` _asfirst_person_character))

(event `self.ReceiveActorEndOverlap`
  (params (OtherActor :type "Actor Object Reference"))
  (bind _asfirst_person_character (cast `/Game/FirstPersonBP/Blueprints/FirstPersonCharacter` OtherActor))
  (set `self.forceMultiplier` 0)
  (set `/Game/FirstPersonBP/Blueprints/FirstPersonCharacter.isOnConveyerBelt` false _asfirst_person_character)
  (`/Game/FirstPersonBP/Blueprints/FirstPersonCharacter.conveyerBeltStatus` _asfirst_person_character))

(event `self.ReceiveTick`
  (params (DeltaSeconds :type "Float (single-precision)"))
  (`CharacterMovementComponent.AddForce` (`Character.CharacterMovement` (stale `self.ReceiveActorBeginOverlap` _asfirst_person_character)) (* (`SceneComponent.GetForwardVector` (`self.BeltPlaceholder`)) (`self.forceMultiplier`))))

(fn `UserConstructionScript`)