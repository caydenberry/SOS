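; Giant door actor that opens once when its linked button is pressed.
; BeginPlay casts the Button reference to the button Blueprint, printing "Fail" if that fails, and Tick polls its IsPressed state until the door opens.
; DoorOpen sets IsOpen, then slides the two door components to new relative locations with MoveComponentTo, the second starting after a short delay and moving more slowly.
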(event `self.ReceiveBeginPlay`
  ;[1 1 1] Making the power work or not
  (bind _asbutton (cast `/Game/assets/blueprints/Interactables/button` (`self.button`))
    (:`CastFailed`
      (`KismetSystemLibrary.PrintString` "Fail"))))

(event `self.ReceiveTick`
  (params (DeltaSeconds :type "Float (single-precision)"))
  ;[1 1 1] Tick
  (if (`self.isOpen`)
    _
    (elif (`/Game/assets/blueprints/Interactables/button.isPressed` (stale `self.ReceiveBeginPlay` _asbutton))
      (`self.DoorOpen`))))

(event `DoorOpen`
  ;[1 1 1] Door Open
  (set `self.isOpen` true)
  (`KismetSystemLibrary.MoveComponentTo` (`self.giant_door2`) (0.0 -50.0 600.0) (struct) false false 2.5)
  (`KismetSystemLibrary.Delay` 0.25)
  (`KismetSystemLibrary.MoveComponentTo` (`self.giant_door`) (0.0 50.0 0.0) (struct) false false 3.5))

(fn `UserConstructionScript`)